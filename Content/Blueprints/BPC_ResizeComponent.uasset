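; Actor component that grows or shrinks its owning actor while a beam is on it.
; StartScale_Event sets the direction and turns scaling on, and StopScale_Event turns it off.
; While active, Tick adds or subtracts GrowAmount from the owner's scale every frame, not scaled by delta time, applying it only while the X axis stays within MinScale and MaxScale.
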(event Custom|StartScale_Event
  (params (bShouldGrow :type Boolean))
  (Variables|Default|SetbShouldGrow bShouldGrow)
  (Variables|Default|SetbIsGettingBeamed true))

(event Custom|StopScale_Event
  (Variables|Default|SetbIsGettingBeamed false))

(event EventBeginPlay)

(event EventTick
  (params (DeltaSeconds :type Float%20%28single-precision%29))
  (if (Variables|Default|GetbIsGettingBeamed)
    (if (Variables|Default|GetbShouldGrow)
      (Variables|Default|SetNewScale (+ (Transformation|GetActorScale3D (Components|GetOwner self)) (Variables|Default|GetgrowAmount)))
      (if (>= (.x (Variables|Default|GetMaxScale)) (.x (Variables|Default|GetNewScale)))
        (Transformation|SetActorScale3D (Components|GetOwner self) (Variables|Default|GetNewScale) :!label _label))
      (else
        (Variables|Default|SetNewScale (+ (Transformation|GetActorScale3D (Components|GetOwner self)) (* (Variables|Default|GetgrowAmount) -1.0)))
        (if (>= (.x (Variables|Default|GetNewScale)) (.x (Variables|Default|GetMinScale)))
          (goto _label))))))