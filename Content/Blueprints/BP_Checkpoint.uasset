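; BP_Checkpoint is a checkpoint actor that sets the player's respawn point when overlapped.
; On the first overlap it casts the other actor to BP_FirstPersonCharacter and copies the RespawnPosition component's world transform into that character's SpawnTransform.
; The DoOnce precedes the cast, so any overlapping actor uses up the checkpoint.
; Debug prints then show the saved location, rotation and scale.
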(event EventBeginPlay)

(event Collision|EventActorBeginOverlap
  (params (OtherActor :type Actor%20Object%20Reference))
  (Utilities|FlowControl|DoOnce false
    (:Completed
      (bind _asbp_first_person_character (Utilities|Casting|CastToBP_FirstPersonCharacter OtherActor))
      (bind _output_get (Variables|/Game/FirstPerson/Blueprints/BP_FirstPersonCharacter.BP_FirstPersonCharacter_C|SetSpawnTransform _asbp_first_person_character (Transformation|GetWorldTransform (Variables|Default|GetRespawnPosition))))
      (Development|PrintString "SpawnPoint Set" true true "(R=0.000000,G=0.660000,B=1.000000,A=1.000000)" 5.0)
      (Development|PrintString (Utilities|String|Append "Position:" (Utilities|String|ToString(Vector) (.Location (Math|Transform|BreakTransform _output_get)))) true true "(R=0.000000,G=0.660000,B=1.000000,A=1.000000)" 5.0)
      (Development|PrintString (Utilities|String|Append "Rotation:" (Utilities|String|ToString(Rotator) (.Rotation (Math|Transform|BreakTransform _output_get)))) true true "(R=0.000000,G=0.660000,B=1.000000,A=1.000000)" 5.0)
      (Development|PrintString (Utilities|String|Append "Scale:" (Utilities|String|ToString(Vector) (.Scale (Math|Transform|BreakTransform _output_get)))) true true "(R=0.000000,G=0.660000,B=1.000000,A=1.000000)" 5.0))))

(event EventTick
  (params (DeltaSeconds :type Float%20%28single-precision%29)))

(fn ConstructionScript)