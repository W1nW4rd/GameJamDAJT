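; Actor component that lets its owner build a signed charge, then grow or shrink by that amount once resizing starts.
; Charge raises or lowers the value within a symmetric limit, flags it when full and shows it on the owner's TextRenderComponent.
; StartResize locks further charging and starts a looping timer that adds the charge to the actor's scale each tick until the max or min scale is reached.
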(event Custom|StartResize
  (Variables|Default|SetbLeverPulled true)
  (if (> (Variables|Default|GetchargeAmount) 0.0)
    (bind _returnvalue (Utilities|Time|SetTimerbyEvent (delegate Custom|Grow) 0.01 true))
    (Variables|Default|SetresizeTimerEvent _returnvalue)
    (elif (< (Variables|Default|GetchargeAmount) 0.0)
      (bind _returnvalue_2 (Utilities|Time|SetTimerbyEvent (delegate Custom|Shrink) 0.01 true))
      (Variables|Default|SetresizeTimerEvent _returnvalue_2))))

(event Custom|Charge
  (params (bIsCharging :type Boolean))
  (if (not (Variables|Default|GetbLeverPulled))
    (if bIsCharging
      (Variables|Default|SetchargeAmount (+ (Variables|Default|GetchargeAmount) (Variables|Default|GetchargeRate)))
      (else
        (Variables|Default|SetchargeAmount (+ (Variables|Default|GetchargeAmount) (* (Variables|Default|GetchargeRate) -1.0)))))
    (if (>= (Variables|Default|GetmaxChargeAmount) (Math|Float|Absolute(Float) (Variables|Default|GetchargeAmount)))
      (Variables|Default|SetchargeAmount (Variables|Default|GetchargeAmount))
      (Development|PrintString "Charging")
      (else
        (if bIsCharging
          (Variables|Default|SetchargeAmount (Variables|Default|GetmaxChargeAmount))
          (else
            (Variables|Default|SetchargeAmount (* (Variables|Default|GetmaxChargeAmount) -1.0))))
        (Development|PrintString "FULL")
        (Variables|Default|SetbIsFull true)))
    (Rendering|Components|TextRender|SetText (Actor|GetComponentbyClass (Components|GetOwner) "/Script/Engine.TextRenderComponent") (Utilities|Text|ToText(Float) (Variables|Default|GetchargeAmount) "HalfToEven"))))

(event Custom|Grow
  (bind _self self)
  (bind _returnvalue (Components|GetOwner _self))
  ;[1 1 1] Grow Event
  (Variables|Default|SetnewScale (+ (Transformation|GetActorScale3D _returnvalue) (Variables|Default|GetchargeAmount)))
  (if (>= (.x (Variables|Default|GetmaxScale)) (.x (Variables|Default|GetnewScale)))
    (Transformation|SetActorScale3D _returnvalue (Variables|Default|GetnewScale))
    (else
      (Transformation|SetActorScale3D _returnvalue (Variables|Default|GetmaxScale))
      (Utilities|Time|ClearandInvalidateTimerbyHandle (Variables|Default|GetresizeTimerEvent)))))

(event Custom|Shrink
  (bind _self self)
  (bind _returnvalue (Components|GetOwner _self))
  ;[1 1 1] Shrink Event
  (Variables|Default|SetnewScale (+ (Transformation|GetActorScale3D _returnvalue) (Variables|Default|GetchargeAmount)))
  (if (>= (.x (Variables|Default|GetnewScale)) (.x (Variables|Default|GetminScale)))
    (Transformation|SetActorScale3D _returnvalue (Variables|Default|GetnewScale))
    (else
      (Transformation|SetActorScale3D _returnvalue (Variables|Default|GetminScale))
      (Utilities|Time|ClearandInvalidateTimerbyHandle (Variables|Default|GetresizeTimerEvent)))))

(event EventBeginPlay)

(event EventTick
  (params (DeltaSeconds :type Float%20%28single-precision%29)))