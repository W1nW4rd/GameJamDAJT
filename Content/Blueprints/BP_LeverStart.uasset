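; BP_LeverStart is an interactable lever that starts resizing on linked charge actors, with a load event that reverts it.
; Interact, once until reloaded, saves ScaleActors' scales, calls StartResize on each ChargeActors' BPC_ChargeComponent and turns the sphere green.
; LoadEvent restores scales and stored charge amounts, clears LeverPulled and re-arms the lever.
; Save leaves ChargeAmount unwired, so it stores default values instead of current charges.
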(event Custom|Interact
  (if (not (Variables|Default|GetbIsActivated))
    (CallFunction|Save)
    (for _array_element (Variables|Default|GetChargeActors)
      (Default|StartResize (Actor|GetComponentbyClass _array_element "/Game/Blueprints/BPC_ChargeComponent.BPC_ChargeComponent_C")))
    (Rendering|Material|SetMaterial (Variables|Default|GetSphere) 0 "/Game/Graphics/Materials/m_Green.m_Green")
    (Variables|Default|SetbIsActivated true)))

(event Custom|LoadEvent
  (CallFunction|Load)
  (Variables|Default|SetbIsActivated false))

(event EventBeginPlay)

(event Collision|EventActorBeginOverlap
  (params (OtherActor :type Actor%20Object%20Reference)))

(event EventTick
  (params (DeltaSeconds :type Float%20%28single-precision%29)))

(fn ConstructionScript)

(fn Save
  (for (_array_element _array_index) (Variables|Default|GetScaleActors)
    (Utilities|Array|SetArrayElem (Variables|Default|GetSavedScaledActors) _array_index (Transformation|GetActorScale3D _array_element) true))
  (for (_array_element_2 _array_index_2) (Variables|Default|GetChargeActors)
    (Utilities|Array|SetArrayElem (Variables|Default|GetSavedChargeActors) _array_index_2 0.0 true)))

(fn Load
  (for (_array_element _array_index) (Variables|Default|GetScaleActors)
    (Transformation|SetActorScale3D _array_element (Utilities|Array|Get(acopy) (Variables|Default|GetSavedScaledActors) _array_index)))
  (for (_array_element_2 _array_index_2) (Variables|Default|GetChargeActors)
    (Variables|/Game/Blueprints/BPC_ChargeComponent.BPC_ChargeComponent_C|SetchargeAmount (Actor|GetComponentbyClass _array_element_2 "/Game/Blueprints/BPC_ChargeComponent.BPC_ChargeComponent_C") (Utilities|Array|Get(acopy) (Variables|Default|GetSavedChargeActors) _array_index_2))
    (Variables|/Game/Blueprints/BPC_ChargeComponent.BPC_ChargeComponent_C|SetbLeverPulled (Actor|GetComponentbyClass _array_element_2 "/Game/Blueprints/BPC_ChargeComponent.BPC_ChargeComponent_C") false)))